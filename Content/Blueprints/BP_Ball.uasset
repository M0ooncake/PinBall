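; BP_Ball is a physics-driven ball actor that is pushed along and pressed toward the table.
; Every Tick applies a default-speed velocity-change impulse to BallMesh, scaled by delta time.
; A Visibility line trace, whose end multiplies the location by a Z-only vector rather than offsetting it, supplies an impact normal.
; A second impulse pushes against that normal, scaled by TableStickyness, without checking for a hit.
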(event `self.ReceiveTick`
  (params (DeltaSeconds :type "Float (single-precision)"))
  (bind _returnvalue (`self.K2_GetActorLocation`))
  (`|ExecutionSequence`
    (:`then_0`
      (`PrimitiveComponent.AddImpulse` (`self.BallMesh`) (* (`self.DefualtSpeed`) DeltaSeconds) "None" true)
      (bind _outhit (`KismetSystemLibrary.LineTraceSingle` _returnvalue (* _returnvalue (0.0 0.0 500.0)) "TraceTypeQuery1"))
      (`PrimitiveComponent.AddImpulse` (`self.BallMesh`) (* (* (`.ImpactNormal` (`GameplayStatics.BreakHitResult` _outhit)) -1.0) (* (`self.TableStickyness`) DeltaSeconds)) "None" false))))

(fn `UserConstructionScript`)