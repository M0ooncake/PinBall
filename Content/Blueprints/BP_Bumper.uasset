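; BP_Bumper is a pinball bumper that reacts when a BP_Ball overlaps it.
; It launches the ball away from its centre with a velocity-change impulse, adds score through PinBallGameMode and spawns an emitter at the mechanism.
; A BumpLerp timeline animates BumperMechanism along its vertical axis.
; The construction script creates and stores a dynamic material instance for the bumper top.
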(event `self.ReceiveActorBeginOverlap`
  (params (OtherActor :type "Actor Object Reference"))
  (bind _asbp_ball (cast `/Game/Blueprints/BP_Ball` OtherActor))
  (`self.Bump` _asbp_ball))

(event `Bump`
  (params (Ball :type "/Game/Blueprints/BP_Ball Object Reference"))
  (`PrimitiveComponent.AddImpulse` (`/Game/Blueprints/BP_Ball.BallMesh` Ball) (* (`KismetMathLibrary.GetDirectionUnitVector` (`self.K2_GetActorLocation`) (`self.K2_GetActorLocation` Ball)) 2500.0) "None" true)
  (bind _aspin_ball_game_mode (cast `/Game/Blueprints/PinBallGameMode` (`GameplayStatics.GetGameMode`))
    (:`then`
      (`/Game/Blueprints/PinBallGameMode.AddScore` _aspin_ball_game_mode 10.0))
    (:`CastFailed`
      _))
  (`GameplayStatics.SpawnEmitterAtLocation` null (`SceneComponent.K2_GetComponentLocation` (`self.BumperMechanism`)))
  (bind (_direction _bumpalpha) (`Timeline|BumpLerp` :!via `PlayFromStart`)
    (:`Update`
      (`SceneComponent.K2_SetRelativeLocation` (`self.BumperMechanism`) (`KismetMathLibrary.VLerp` (0.0 0.0 0.0) (0.0 0.0 -70.0) _bumpalpha) false false))))

(fn `UserConstructionScript`
  (bind _returnvalue (`PrimitiveComponent.CreateDynamicMaterialInstance` (`self.BumperMesh`) 1 null "None"))
  (set `self.BumperTopMID` _returnvalue))