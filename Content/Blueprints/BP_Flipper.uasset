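; BP_Flipper is a left or right flipper, likely for pinball, that swings between a resting and a flipped rotation.
; The construction script picks mirrored start and end angles from FlipType, applies the starting rotation, and flips the mesh with negative X scale for the right side.
; Flip and Flop events use MoveComponentTo to rotate the Flipper component to either angle over FlipTime.
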(event `Flip`
  (`KismetSystemLibrary.MoveComponentTo` (`self.Flipper`) (0.0 0.0 0.0) (`self.EndingRotation`) false false (`self.FlipTime`)))

(event `Flop`
  (`KismetSystemLibrary.MoveComponentTo` (`self.Flipper`) (0.0 0.0 0.0) (`self.StartingRotation`) false false (`self.FlipTime`)))

(fn `UserConstructionScript`
  (set `self.StartingRotation` (select `/Game/Blueprints/E_FlipTypes` (`self.FlipType`) :`NewEnumerator0` (struct :`Yaw` 20.0) :`NewEnumerator1` (struct :`Yaw` -20.0) :!type "Rotator Structure"))
  (set `self.EndingRotation` (select `/Game/Blueprints/E_FlipTypes` (`self.FlipType`) :`NewEnumerator0` (struct :`Yaw` -20.0) :`NewEnumerator1` (struct :`Yaw` 20.0) :!type "Rotator Structure"))
  (`SceneComponent.K2_SetRelativeRotation` (`self.Flipper`) (`self.StartingRotation`) false false)
  (switch `/Game/Blueprints/E_FlipTypes` (`self.FlipType`)
    (:`NewEnumerator1`
      (`SceneComponent.SetRelativeScale3D` (`self.Flipper`) (-1.0 1.0 1.0)))))