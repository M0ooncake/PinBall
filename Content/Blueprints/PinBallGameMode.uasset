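; PinBallGameMode is the pinball game mode that spawns balls and tracks how many remain.
; On BeginPlay it spawns a BP_Ball at the spawn location provided by the first BP_Plunger found in the level.
; Each ball's OnDestroyed event is bound to a handler that spawns a replacement and decrements BallsRemaining while any are left.
; No action follows when the count reaches zero.
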(event `SpawnBall`
  (bind _outactors (`GameplayStatics.GetAllActorsOfClass` "/Game/Blueprints/BP_Plunger.BP_Plunger_C"))
  (bind _returnvalue (`|SpawnActorFromClass` "/Game/Blueprints/BP_Ball.BP_Ball_C" (`KismetMathLibrary.MakeTransform` (`/Game/Blueprints/BP_Plunger.GetBallSpawnLocation` (`|GetArrayItem` _outactors))) "Undefined" "MultiplyWithRoot" null null))
  (add `self.OnDestroyed` _returnvalue (delegate `OnBallDestroyed`)))

(event `self.ReceiveBeginPlay`
  (`self.SpawnBall`))

(event `OnBallDestroyed` :!signature `self.OnDestroyed`
  (params (DestroyedActor :type "Actor Object Reference"))
  (if (> (`self.BallsRemaining`) 0)
    (`self.SpawnBall`)
    (`/Engine/EditorBlueprintResources/StandardMacros.DecrementInt` (`self.BallsRemaining`))))

(fn `UserConstructionScript`)